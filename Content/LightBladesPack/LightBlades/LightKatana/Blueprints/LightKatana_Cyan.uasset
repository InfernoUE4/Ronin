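; Cyan light katana Blueprint that switches its blade between off, light blade and unstable blade looks.
; On/Off events swap the LightKatanaBlade material in slot 0 after a short delay, and light blade ignition briefly flickers back to the base material.
; Each event first checks the mesh's EnableMaterialParameterCaching flag and, when true, only sets IsLightBladeOff or IsUnstableBladeOff instead of swapping materials.
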(event `OnLightBlade`
  (bind _lightkatana_blade (`self.LightKatana_Blade`))
  (bind _lightkatana_blade_2 (`self.LightKatana_Blade`))
  ;[1 1 1] Turn On/Off LightBlade Cyan
  (if (`MeshComponent.bEnableMaterialParameterCaching` _lightkatana_blade)
    (set `self.IsLightBladeOff?` true)
    (else
      (`KismetSystemLibrary.Delay` 0.5)
      (`PrimitiveComponent.SetMaterial` _lightkatana_blade 0 "/Game/LightBladesPack/LightBlades/BladesMaterial/LightBladesMaterials/LightBlade_Cyan_Material.LightBlade_Cyan_Material")
      (`KismetSystemLibrary.Delay` 0.3)
      (`PrimitiveComponent.SetMaterial` _lightkatana_blade_2 0 "/Game/LightBladesPack/LightBlades/LightKatana/Materials/LightKatana_Blade_Material.LightKatana_Blade_Material")
      (`KismetSystemLibrary.Delay` 0.01)
      (`PrimitiveComponent.SetMaterial` _lightkatana_blade_2 0 "/Game/LightBladesPack/LightBlades/BladesMaterial/LightBladesMaterials/LightBlade_Cyan_Material.LightBlade_Cyan_Material"))))

(event `OffLightBlade`
  (bind _lightkatana_blade (`self.LightKatana_Blade`))
  ;[1 1 1] Turn On/Off LightBlade Cyan
  (if (`MeshComponent.bEnableMaterialParameterCaching` _lightkatana_blade)
    (set `self.IsLightBladeOff?` false)
    (else
      (`KismetSystemLibrary.Delay` 0.5)
      (`PrimitiveComponent.SetMaterial` _lightkatana_blade 0 "/Game/LightBladesPack/LightBlades/LightKatana/Materials/LightKatana_Blade_Material.LightKatana_Blade_Material"))))

(event `OnUnstableBlade`
  (bind _lightkatana_blade (`self.LightKatana_Blade`))
  ;[1 1 1] Turn On/Off UnstableBlade Cyan
  (if (`MeshComponent.bEnableMaterialParameterCaching` _lightkatana_blade)
    (set `self.IsUnstableBladeOff?` true)
    (else
      (`KismetSystemLibrary.Delay` 0.5)
      (`PrimitiveComponent.SetMaterial` _lightkatana_blade 0 "/Game/LightBladesPack/LightBlades/BladesMaterial/UnstableBladesMaterials/UnstableBlade_Cyan_Material.UnstableBlade_Cyan_Material"))))

(event `OffUnstableBlade`
  (bind _lightkatana_blade (`self.LightKatana_Blade`))
  ;[1 1 1] Turn On/Off UnstableBlade Cyan
  (if (`MeshComponent.bEnableMaterialParameterCaching` _lightkatana_blade)
    (set `self.IsUnstableBladeOff?` false)
    (else
      (`KismetSystemLibrary.Delay` 0.5)
      (`PrimitiveComponent.SetMaterial` _lightkatana_blade 0 "/Game/LightBladesPack/LightBlades/LightKatana/Materials/LightKatana_Blade_Material.LightKatana_Blade_Material"))))

(fn `UserConstructionScript`)