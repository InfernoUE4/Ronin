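; Magenta light knife Blueprint with events that turn its light blade and unstable blade looks on and off.
; Each event swaps the blade mesh's material after short delays between the plain knife material and a magenta one, with a brief flicker on light blade ignition.
; If the blade's EnableMaterialParameterCaching is set, events only write IsLightBladeOff or IsUnstableBladeOff, true for On and false for Off, skipping the swap.
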(event `OnLightBlade`
  (bind _lightknife_blade (`self.LightKnife_Blade`))
  (bind _lightknife_blade_2 (`self.LightKnife_Blade`))
  ;[1 1 1] Turn On/Off LightBlade Magenta
  (if (`MeshComponent.bEnableMaterialParameterCaching` _lightknife_blade_2)
    (set `self.IsLightBladeOff?` true)
    (else
      (`KismetSystemLibrary.Delay` 0.5)
      (`PrimitiveComponent.SetMaterial` _lightknife_blade_2 0 "/Game/LightBladesPack/LightBlades/BladesMaterial/LightBladesMaterials/LightBlade_Magenta_Material.LightBlade_Magenta_Material")
      (`KismetSystemLibrary.Delay` 0.3)
      (`PrimitiveComponent.SetMaterial` _lightknife_blade 0 "/Game/LightBladesPack/LightBlades/LightKnife/Materials/LightKnife_Blade_Material.LightKnife_Blade_Material")
      (`KismetSystemLibrary.Delay` 0.01)
      (`PrimitiveComponent.SetMaterial` _lightknife_blade 0 "/Game/LightBladesPack/LightBlades/BladesMaterial/LightBladesMaterials/LightBlade_Magenta_Material.LightBlade_Magenta_Material"))))

(event `OffLightBlade`
  (bind _lightknife_blade (`self.LightKnife_Blade`))
  ;[1 1 1] Turn On/Off LightBlade Magenta
  (if (`MeshComponent.bEnableMaterialParameterCaching` _lightknife_blade)
    (set `self.IsLightBladeOff?` false)
    (else
      (`KismetSystemLibrary.Delay` 0.5)
      (`PrimitiveComponent.SetMaterial` _lightknife_blade 0 "/Game/LightBladesPack/LightBlades/LightKnife/Materials/LightKnife_Blade_Material.LightKnife_Blade_Material"))))

(event `OnUnstableBlade`
  (bind _lightknife_blade (`self.LightKnife_Blade`))
  ;[1 1 1] Turn On/Off UnstableBlade Magenta
  (if (`MeshComponent.bEnableMaterialParameterCaching` _lightknife_blade)
    (set `self.IsUnstableBladeOff?` true)
    (else
      (`KismetSystemLibrary.Delay` 0.5)
      (`PrimitiveComponent.SetMaterial` _lightknife_blade 0 "/Game/LightBladesPack/LightBlades/BladesMaterial/UnstableBladesMaterials/UnstableBlade_Magenta_Material.UnstableBlade_Magenta_Material"))))

(event `OffUnstableBlade`
  (bind _lightknife_blade (`self.LightKnife_Blade`))
  ;[1 1 1] Turn On/Off UnstableBlade Magenta
  (if (`MeshComponent.bEnableMaterialParameterCaching` _lightknife_blade)
    (set `self.IsUnstableBladeOff?` false)
    (else
      (`KismetSystemLibrary.Delay` 0.5)
      (`PrimitiveComponent.SetMaterial` _lightknife_blade 0 "/Game/LightBladesPack/LightBlades/LightKnife/Materials/LightKnife_Blade_Material.LightKnife_Blade_Material"))))

(fn `UserConstructionScript`)