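; Dark variant of the LightShuriken Blueprint, with events that switch its blade's light and unstable effects on and off.
; Each event checks the blade mesh's EnableMaterialParameterCaching: if set, it only updates an Off flag, otherwise it swaps slot 0's material after a delay.
; Light-on flickers through dark, default and dark materials, unstable-on applies its own dark material, and both off events restore the default blade material.
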(event `OnLightBlade`
  (bind _lightshuriken_blade (`self.LightShuriken_Blade`))
  ;[1 1 1] Turn On/Off LightBlade Dark
  (if (`MeshComponent.bEnableMaterialParameterCaching` (`self.LightShuriken_Blade`))
    (set `self.IsLightBladeOff?` true)
    (else
      (`KismetSystemLibrary.Delay` 0.5)
      (`PrimitiveComponent.SetMaterial` (`self.LightShuriken_Blade`) 0 "/Game/LightBladesPack/LightBlades/BladesMaterial/LightBladesMaterials/LightBlade_Dark_Material.LightBlade_Dark_Material")
      (`KismetSystemLibrary.Delay` 0.3)
      (`PrimitiveComponent.SetMaterial` _lightshuriken_blade 0 "/Game/LightBladesPack/LightBlades/LightShuriken/Materials/LightShuriken_Blade_Material.LightShuriken_Blade_Material")
      (`KismetSystemLibrary.Delay` 0.01)
      (`PrimitiveComponent.SetMaterial` _lightshuriken_blade 0 "/Game/LightBladesPack/LightBlades/BladesMaterial/LightBladesMaterials/LightBlade_Dark_Material.LightBlade_Dark_Material"))))

(event `OffLightBlade`
  ;[1 1 1] Turn On/Off LightBlade Dark
  (if (`MeshComponent.bEnableMaterialParameterCaching` (`self.LightShuriken_Blade`))
    (set `self.IsLightBladeOff?` false)
    (else
      (`KismetSystemLibrary.Delay` 0.5)
      (`PrimitiveComponent.SetMaterial` (`self.LightShuriken_Blade`) 0 "/Game/LightBladesPack/LightBlades/LightShuriken/Materials/LightShuriken_Blade_Material.LightShuriken_Blade_Material"))))

(event `OnUnstableBlade`
  ;[1 1 1] Turn On/Off UnstableBlade Dark
  (if (`MeshComponent.bEnableMaterialParameterCaching` (`self.LightShuriken_Blade`))
    (set `self.IsUnstableBladeOff?` true)
    (else
      (`KismetSystemLibrary.Delay` 0.5)
      (`PrimitiveComponent.SetMaterial` (`self.LightShuriken_Blade`) 0 "/Game/LightBladesPack/LightBlades/BladesMaterial/UnstableBladesMaterials/UnstableBlade_Dark_Material.UnstableBlade_Dark_Material"))))

(event `OffUnstableBlade`
  ;[1 1 1] Turn On/Off UnstableBlade Dark
  (if (`MeshComponent.bEnableMaterialParameterCaching` (`self.LightShuriken_Blade`))
    (set `self.IsUnstableBladeOff?` false)
    (else
      (`KismetSystemLibrary.Delay` 0.5)
      (`PrimitiveComponent.SetMaterial` (`self.LightShuriken_Blade`) 0 "/Game/LightBladesPack/LightBlades/LightShuriken/Materials/LightShuriken_Blade_Material.LightShuriken_Blade_Material"))))

(fn `UserConstructionScript`)