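; Red light spear weapon Blueprint with events to switch its two blade meshes on and off in a steady or unstable red style.
; Each event waits briefly, then swaps both blades between the red glow materials and the plain blade material, with a short flicker when the steady blade ignites.
; If the first blade has material parameter caching enabled, events only set that style's "off" flag, true for On and false for Off.
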(event `OnLightBlade`
  (bind _lightspear_blade (`self.LightSpear_Blade`))
  ;[1 1 1] Turn On/Off LightBlade Red
  (if (`MeshComponent.bEnableMaterialParameterCaching` (`self.LightSpear_Blade`))
    (set `self.IsLightBladeOff?` true)
    (else
      (`KismetSystemLibrary.Delay` 0.5)
      (`PrimitiveComponent.SetMaterial` (`self.LightSpear_Blade2`) 0 "/Game/LightBladesPack/LightBlades/BladesMaterial/LightBladesMaterials/LightBlade_Red_Material.LightBlade_Red_Material")
      (`PrimitiveComponent.SetMaterial` (`self.LightSpear_Blade`) 0 "/Game/LightBladesPack/LightBlades/BladesMaterial/LightBladesMaterials/LightBlade_Red_Material.LightBlade_Red_Material")
      (`KismetSystemLibrary.Delay` 0.3)
      (`PrimitiveComponent.SetMaterial` _lightspear_blade 0 "/Game/LightBladesPack/LightBlades/LightSpear/Materials/LightSpear_Blade_Material.LightSpear_Blade_Material")
      (`PrimitiveComponent.SetMaterial` (`self.LightSpear_Blade2`) 0 "/Game/LightBladesPack/LightBlades/LightSpear/Materials/LightSpear_Blade_Material.LightSpear_Blade_Material")
      (`KismetSystemLibrary.Delay` 0.01)
      (`PrimitiveComponent.SetMaterial` _lightspear_blade 0 "/Game/LightBladesPack/LightBlades/BladesMaterial/LightBladesMaterials/LightBlade_Red_Material.LightBlade_Red_Material")
      (`PrimitiveComponent.SetMaterial` (`self.LightSpear_Blade2`) 0 "/Game/LightBladesPack/LightBlades/BladesMaterial/LightBladesMaterials/LightBlade_Red_Material.LightBlade_Red_Material"))))

(event `OffLightBlade`
  (bind _lightspear_blade (`self.LightSpear_Blade`))
  ;[1 1 1] Turn On/Off LightBlade Red
  (if (`MeshComponent.bEnableMaterialParameterCaching` _lightspear_blade)
    (set `self.IsLightBladeOff?` false)
    (else
      (`KismetSystemLibrary.Delay` 0.5)
      (`PrimitiveComponent.SetMaterial` _lightspear_blade 0 "/Game/LightBladesPack/LightBlades/LightSpear/Materials/LightSpear_Blade_Material.LightSpear_Blade_Material")
      (`PrimitiveComponent.SetMaterial` (`self.LightSpear_Blade2`) 0 "/Game/LightBladesPack/LightBlades/LightSpear/Materials/LightSpear_Blade_Material.LightSpear_Blade_Material"))))

(event `OnUnstableBlade`
  (bind _lightspear_blade (`self.LightSpear_Blade`))
  ;[1 1 1] Turn On/Off UnstableBlade Red
  (if (`MeshComponent.bEnableMaterialParameterCaching` _lightspear_blade)
    (set `self.IsUnstableBladeOff?` true)
    (else
      (`KismetSystemLibrary.Delay` 0.5)
      (`PrimitiveComponent.SetMaterial` _lightspear_blade 0 "/Game/LightBladesPack/LightBlades/BladesMaterial/UnstableBladesMaterials/UnstableBlade_Red_Material.UnstableBlade_Red_Material")
      (`PrimitiveComponent.SetMaterial` (`self.LightSpear_Blade2`) 0 "/Game/LightBladesPack/LightBlades/BladesMaterial/UnstableBladesMaterials/UnstableBlade_Red_Material.UnstableBlade_Red_Material"))))

(event `OffUnstableBlade`
  (bind _lightspear_blade (`self.LightSpear_Blade`))
  ;[1 1 1] Turn On/Off UnstableBlade Red
  (if (`MeshComponent.bEnableMaterialParameterCaching` _lightspear_blade)
    (set `self.IsUnstableBladeOff?` false)
    (else
      (`KismetSystemLibrary.Delay` 0.5)
      (`PrimitiveComponent.SetMaterial` _lightspear_blade 0 "/Game/LightBladesPack/LightBlades/LightSpear/Materials/LightSpear_Blade_Material.LightSpear_Blade_Material")
      (`PrimitiveComponent.SetMaterial` (`self.LightSpear_Blade2`) 0 "/Game/LightBladesPack/LightBlades/LightSpear/Materials/LightSpear_Blade_Material.LightSpear_Blade_Material"))))

(fn `UserConstructionScript`)