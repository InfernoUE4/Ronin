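; BP_AbilityTreeNode is an ability tree node that grants an ability to the character's BPCAbilities component when activated.
; Activate switches on node type and upgrade level, with only the base Dash case shown building an ability struct.
; UpdateAbilitiesList finds an entry with the same TreeNodeType and overwrites it, or appends otherwise.
; Its index check is strictly above zero, so a match in the first slot is appended again.
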(fn `Ability == Ability`
  (params (` ` :type "/Game/Blueprints/Components/Abilities/ST_Ability Structure") (`  ` :type "/Game/Blueprints/Components/Abilities/ST_Ability Structure"))
  (returns (`   ` :type Boolean))
  (return (`|EnumEquality` (`.TreeNodeType_5_EB3FB2D843745C8CD50F1197DF011427` (break `/Game/Blueprints/Components/Abilities/ST_Ability` ` `)) (`.TreeNodeType_5_EB3FB2D843745C8CD50F1197DF011427` (break `/Game/Blueprints/Components/Abilities/ST_Ability` `  `)))))

(fn `Activate`
  (switch `/Game/Blueprints/Components/Abilities/ETreeNodeType` (`self.NodeType`)
    (:`NewEnumerator0`
      (switch `int` (`self.Upgrade`)
        (:`0`
          (`self.UpdateAbilitiesList` (make `/Game/Blueprints/Components/Abilities/ST_Ability` "NewEnumerator0" 1 1000.0 1.0 -1.0 5.0 0.0)))))))

(fn `GetAbilityListIndex`
  (params (Ability :type "/Game/Blueprints/Components/Abilities/ST_Ability Structure"))
  (returns (` ` :type Integer))
  (for (_array_element _array_index) (`/Game/Blueprints/Components/Abilities/BPC_Abilities.AvailableAbilities` (`/Game/Blueprints/Core/BP_Character.BPC_Abilities` (`self.Character`)))
    (if (`self.Ability == Ability` _array_element Ability)
      (return _array_index)))
  (return -1))

(fn `UpdateAbilitiesList`
  (params (Ability :type "/Game/Blueprints/Components/Abilities/ST_Ability Structure"))
  (returns (` ` :type Boolean))
  (bind _availableabilities (`/Game/Blueprints/Components/Abilities/BPC_Abilities.AvailableAbilities` (`/Game/Blueprints/Core/BP_Character.BPC_Abilities` (`self.Character`))))
  (bind __ (`self.GetAbilityListIndex` Ability))
  (if (> __ 0)
    (`KismetArrayLibrary.Array_Set` _availableabilities __ Ability)
    (else
      (`KismetArrayLibrary.Array_Add` _availableabilities Ability)))
  (return false))