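; Grappling hook actor that pulls the player toward itself, with a cable attached to the player.
; Each tick it launches the player along the direction to the hook while a check against its Normal passes, otherwise destroying itself.
; Player overlap with its sphere closes the pull gate and opens a damping gate.
; Damping gradually bleeds off player velocity and destroys the hook once speed is low.
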(event `self.ReceiveBeginPlay`
  (`CableComponent.SetAttachEndTo` (`self.Cable`) (`GameplayStatics.GetPlayerCharacter` 0) "None" "None"))

(event `self.ReceiveTick`
  (params (DeltaSeconds :type "Float (single-precision)"))
  (bind _returnvalue (`GameplayStatics.GetPlayerCharacter` 0))
  (bind _returnvalue_2 (`self.GetVelocity` _returnvalue))
  (if (or (> (`KismetMathLibrary.Abs` (- (.x (`self.Normal`)) (.x (`KismetMathLibrary.GetForwardVector` (`KismetMathLibrary.FindLookAtRotation` (`self.K2_GetActorLocation` (`GameplayStatics.GetPlayerCharacter` 0)) (`self.K2_GetActorLocation`)))))) 0.9) (> (`KismetMathLibrary.Abs` (- (.y (`self.Normal`)) (.y (`KismetMathLibrary.GetForwardVector` (`KismetMathLibrary.FindLookAtRotation` (`self.K2_GetActorLocation` (`GameplayStatics.GetPlayerCharacter` 0)) (`self.K2_GetActorLocation`)))))) 0.9) (> (`KismetMathLibrary.Abs` (- (.z (`self.Normal`)) (.z (`KismetMathLibrary.GetForwardVector` (`KismetMathLibrary.FindLookAtRotation` (`self.K2_GetActorLocation` (`GameplayStatics.GetPlayerCharacter` 0)) (`self.K2_GetActorLocation`)))))) 0.9))
    (`|ExecutionSequence`
      (:`then_0`
        (`/Engine/EditorBlueprintResources/StandardMacros.Gate` false :!label _label
          (:`Exit`
            (`Character.LaunchCharacter` _returnvalue (* (`KismetMathLibrary.GetForwardVector` (`KismetMathLibrary.FindLookAtRotation` (`self.K2_GetActorLocation` _returnvalue) (`self.K2_GetActorLocation`))) 20.0) false false))))
      (:`then_1`
        (`/Engine/EditorBlueprintResources/StandardMacros.Gate` true :!label _label_2
          (:`Exit`
            (`Character.LaunchCharacter` _returnvalue (* _returnvalue_2 0.99) true true)
            (if (<= (`KismetMathLibrary.VSize` _returnvalue_2) 300.0)
              (`self.K2_DestroyActor`))))))
    (else
      (`self.K2_DestroyActor`))))

(event `self.Sphere.OnComponentBeginOverlap`
  (params (OverlappedComponent :type "PrimitiveComponent Object Reference") (OtherActor :type "Actor Object Reference") (OtherComp :type "PrimitiveComponent Object Reference") (OtherBodyIndex :type Integer) (bFromSweep :type Boolean) (SweepResult :type "HitResult Structure (by ref)"))
  (if (== OtherActor (`GameplayStatics.GetPlayerCharacter` 0))
    (`|ExecutionSequence`
      (:`then_0`
        (goto _label :!via `Close`))
      (:`then_1`
        (goto _label_2 :!via `Open`)))))

(fn `UserConstructionScript`)