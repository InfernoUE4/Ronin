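; BP_GrapplingHookProjectile is the in-flight hook of the grappling hook ability, with a cable attached back to the first player character.
; Each tick it runs a short forward sphere trace on the Visibility channel, with debug drawing left on.
; On hitting anything but the player, it spawns BP_GrapplingHook at its own transform, passing the hit normal, then destroys itself.
; If nothing is hit, it expires after a brief delay.
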(event `self.ReceiveBeginPlay`
  (`CableComponent.SetAttachEndTo` (`self.Cable`) (`GameplayStatics.GetPlayerCharacter` 0) "None" "None")
  (`KismetSystemLibrary.Delay` 2.0)
  (`self.K2_DestroyActor`))

(event `self.ReceiveTick`
  (params (DeltaSeconds :type "Float (single-precision)"))
  (bind _returnvalue (`self.K2_GetActorLocation`))
  (bind (_outhit _returnvalue_2) (`KismetSystemLibrary.SphereTraceSingle` :`Start` _returnvalue :`End` (+ _returnvalue (* (`self.GetActorForwardVector`) 25.0)) :`Radius` 25.0 :`TraceChannel` "TraceTypeQuery1" :`DrawDebugType` "ForDuration"))
  (if _returnvalue_2
    (bind (_bblockinghit _binitialoverlap _time _distance _location _impactpoint _normal _impactnormal _physmat _hitactor) (`GameplayStatics.BreakHitResult` _outhit))
    (if (!= _hitactor (`GameplayStatics.GetPlayerCharacter` 0))
      (`|SpawnActorFromClass` "/Game/Blueprints/Components/Abilities/Actives/GrapplingHook/BP_GrapplingHook.BP_GrapplingHook_C" (`self.GetTransform`) "Undefined" "OverrideRootScale" null _normal null)
      (`self.K2_DestroyActor`))))

(fn `UserConstructionScript`)