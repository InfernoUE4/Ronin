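; Clone actor for an active ability that dashes forward, then lingers until its health runs out.
; A looping timer moves it along traced ground, stopping after two seconds, at missing ground or at steep upward angles.
; After seven seconds it repeatedly damages itself and is destroyed below zero health.
; A material parameter collection drives opacity, animated by a timeline on spawn and set to health fraction on damage.
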(event `Tick`
  (bind _returnvalue (+ (`self.K2_GetActorLocation`) (0.0 0.0 96.0)))
  (`|ExecutionSequence`
    (:`then_0`
      (`/Engine/EditorBlueprintResources/StandardMacros.Gate` false :!label _label
        (:`Exit`
          (set `MovementComponent.Velocity` (* (`self.GetActorForwardVector`) 900.0) (`self.CharacterMovement`))
          (bind (_outhit _returnvalue_2) (`KismetSystemLibrary.LineTraceSingle` _returnvalue (+ _returnvalue (* (`self.GetActorForwardVector`) 10.0)) "TraceTypeQuery1"))
          (bind (_bblockinghit _binitialoverlap _time _distance _location _impactpoint _normal _impactnormal _physmat _hitactor _hitcomponent _hitbonename _hititem _faceindex _tracestart _traceend) (`GameplayStatics.BreakHitResult` _outhit))
          (bind _returnvalue_3 (select `bool` _returnvalue_2 :`false` _traceend :`true` _impactpoint))
          (bind (_outhit_2 _returnvalue_4) (`KismetSystemLibrary.LineTraceSingle` _returnvalue_3 (- _returnvalue_3 (0.0 0.0 400.0)) "TraceTypeQuery1"))
          (if _returnvalue_4
            (bind _returnvalue_5 (+ (`.ImpactPoint` (`GameplayStatics.BreakHitResult` _outhit_2)) (0.0 0.0 96.0)))
            (if (or (> (.roll (`KismetMathLibrary.FindLookAtRotation` _returnvalue _returnvalue_5)) 30.0) (> (.pitch (`KismetMathLibrary.FindLookAtRotation` _returnvalue _returnvalue_5)) 30.0))
              (`|ExecutionSequence` :!label _label_2
                (:`then_0`
                  (set `MovementComponent.Velocity` (0.0 0.0 0.0) (`self.CharacterMovement`) :!label _label_3)
                  (goto _label :!via `Close`))
                (:`then_1`
                  (`KismetSystemLibrary.PrintString` "Ended")))
              (else
                (`self.K2_SetActorLocation` _returnvalue_5)))
            (else
              (goto _label_2))))))
    (:`then_1`
      (`/Engine/EditorBlueprintResources/StandardMacros.Gate` true :!label _label_4
        (:`Exit`
          (`self.TakeDamage` 2.0 self "NewEnumerator3"))))))

(event `self.ReceiveBeginPlay`
  (`|ExecutionSequence`
    (:`then_0`
      (`KismetSystemLibrary.Delay` 2.0)
      (goto _label_3))
    (:`then_1`
      (`KismetSystemLibrary.Delay` 7.0)
      (goto _label_4 :!via `Open`))
    (:`then_2`
      (bind (_direction _opacity) (`Timeline|Opacity` :!via `PlayFromStart`)
        (:`Update`
          (`KismetMaterialLibrary.SetScalarParameterValue` "/Game/Blueprints/Components/Abilities/Actives/Invisibility/MPC_Invisibility_Clone.MPC_Invisibility_Clone" "Opacity" _opacity))))
    (:`then_3`
      (`KismetSystemLibrary.K2_SetTimerDelegate` (delegate `Tick`) 0.01 true))))

(event `self.TakeDamage`
  (params (Amount :type "Float (single-precision)") (Inflictor :type "Actor Object Reference") (DamageType :type "/Game/Blueprints/Combat/EDamageType Enum" :default "NewEnumerator0"))
  (bind _result (`/Engine/EditorBlueprintResources/StandardMacros.Float -=` (`self.CurrentHealth`) Amount)
    (:`  `
      (`KismetMaterialLibrary.SetScalarParameterValue` "/Game/Blueprints/Components/Abilities/Actives/Invisibility/MPC_Invisibility_Clone.MPC_Invisibility_Clone" "Opacity" (/ _result (`self.MaxHealth`)))
      (if (< _result 0.0)
        (`self.K2_DestroyActor`)))))

(fn `UserConstructionScript`
  (set `self.CurrentHealth` (`self.MaxHealth`)))