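; BP_SlowField is a temporary area-effect actor under the active abilities that slows time for actors inside it.
; On BeginPlay it sets a fixed lifespan and activates its Niagara effect.
; Its Sphere overlap events lower CustomTimeDilation on entering actors that implement BPI_TimeControl and set it back to normal speed when they leave.
; The interface serves only as an opt-in filter, as none of its functions are called.
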(event `self.ReceiveBeginPlay`
  (`self.SetLifeSpan` 60.0)
  (`ActorComponent.Activate` (`self.Niagara`) false))

(event `self.Sphere.OnComponentBeginOverlap`
  (params (OverlappedComponent :type "PrimitiveComponent Object Reference") (OtherActor :type "Actor Object Reference") (OtherComp :type "PrimitiveComponent Object Reference") (OtherBodyIndex :type Integer) (bFromSweep :type Boolean) (SweepResult :type "HitResult Structure (by ref)"))
  (if (`KismetSystemLibrary.DoesImplementInterface` OtherActor "/Game/Blueprints/Components/Abilities/Ultimates/Rewind/BPI_TimeControl.BPI_TimeControl_C")
    (set `Actor.CustomTimeDilation` 0.25 OtherActor)))

(event `self.Sphere.OnComponentEndOverlap`
  (params (OverlappedComponent :type "PrimitiveComponent Object Reference") (OtherActor :type "Actor Object Reference") (OtherComp :type "PrimitiveComponent Object Reference") (OtherBodyIndex :type Integer))
  (if (`KismetSystemLibrary.DoesImplementInterface` OtherActor "/Game/Blueprints/Components/Abilities/Ultimates/Rewind/BPI_TimeControl.BPI_TimeControl_C")
    (set `Actor.CustomTimeDilation` 1.0 OtherActor)))

(fn `UserConstructionScript`)