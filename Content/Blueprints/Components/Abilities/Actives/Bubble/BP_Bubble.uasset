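; Bubble actor for an active ability that decays over time and can be depleted by damage.
; Every tick it damages itself by a fixed amount, not scaled by delta time, so its lifetime depends on frame rate.
; TakeDamage subtracts from Health, sets the sphere's dynamic material opacity to the health ratio, and destroys the actor below zero.
; The construction script creates that material and fills Health.
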(event `self.ReceiveTick`
  (params (DeltaSeconds :type "Float (single-precision)"))
  (`self.TakeDamage` 1.25 self "NewEnumerator3"))

(event `self.TakeDamage`
  (params (Amount :type "Float (single-precision)") (Inflictor :type "Actor Object Reference") (DamageType :type "/Game/Blueprints/Combat/EDamageType Enum" :default "NewEnumerator0"))
  (bind _health (`self.Health`))
  (bind _result (`/Engine/EditorBlueprintResources/StandardMacros.Float -=` _health Amount)
    (:`  `
      (`MaterialInstanceDynamic.SetScalarParameterValue` (`self.Material`) "Opacity" (/ _health (`self.MaxHealth`)))
      (if (< _result 0.0)
        (`self.K2_DestroyActor`)))))

(fn `UserConstructionScript`
  (bind _returnvalue (`KismetMaterialLibrary.CreateDynamicMaterialInstance` "/Game/Blueprints/Components/Abilities/Actives/Bubble/M_Bubble.M_Bubble"))
  (bind _output_get (set `self.Material` _returnvalue))
  (`MaterialInstanceDynamic.SetScalarParameterValue` _output_get "Opacity" 1.0)
  (`PrimitiveComponent.SetMaterial` (`self.Sphere`) 0 (`self.Material`))
  (set `self.Health` (`self.MaxHealth`)))