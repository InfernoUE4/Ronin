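; Physics-simulated static mesh actor that can be rewound in time, with a configurable mesh and materials.
; Each tick it records its world transform and linear and angular velocities, packing both velocities into one transform's location and scale.
; While Rewind is active, it pops these histories newest-first to restore motion until Forward resumes recording.
; Oldest samples are dropped once the player BP_Character's StartClearingOriginalTimePoints flag is set, capping history length.
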(event `/Game/Blueprints/Components/Abilities/Ultimates/Rewind/BPI_TimeControl.Rewind`
  (set `self.Rewinding?` true))

(event `/Game/Blueprints/Components/Abilities/Ultimates/Rewind/BPI_TimeControl.Forward`
  (set `self.Rewinding?` false))

(event `self.ReceiveTick`
  (params (DeltaSeconds :type "Float (single-precision)"))
  (bind _actortransforms (`self.ActorTransforms`))
  (bind _actorvelocities (`self.ActorVelocities`))
  (bind _staticmesh (`self.StaticMesh`))
  (bind _actorvelocities_2 (`self.ActorVelocities`))
  (bind _actortransforms_2 (`self.ActorTransforms`))
  (bind _actortransforms_3 (`self.ActorTransforms`))
  (bind _staticmesh_2 (`self.StaticMesh`))
  (bind _actorvelocities_3 (`self.ActorVelocities`))
  (bind _returnvalue (`KismetArrayLibrary.Array_LastIndex` _actortransforms))
  (bind _returnvalue_2 (`KismetArrayLibrary.Array_LastIndex` _actortransforms_3))
  (bind _returnvalue_3 (`KismetArrayLibrary.Array_LastIndex` _actorvelocities))
  (bind _returnvalue_4 (`KismetArrayLibrary.Array_LastIndex` _actorvelocities_2))
  (`|ExecutionSequence`
    (:`then_0`
      (if (`self.Rewinding?`)
        (if (> _returnvalue_2 -1)
          (`SceneComponent.K2_SetWorldTransform` (`self.StaticMesh`) (`|GetArrayItem` _actortransforms_3 _returnvalue_2) false false)
          (if (> _returnvalue 0)
            (`KismetArrayLibrary.Array_Remove` _actortransforms _returnvalue)
            (else
              (`KismetArrayLibrary.Array_Clear` _actortransforms))))
        (else
          (`KismetArrayLibrary.Array_Add` _actortransforms_2 (`SceneComponent.K2_GetComponentToWorld` (`self.StaticMesh`)))
          (if (`self.ShouldDelete0thTerm`)
            (`KismetArrayLibrary.Array_Remove` _actortransforms_2)))))
    (:`then_1`
      (if (`self.Rewinding?`)
        (if (> _returnvalue_4 -1)
          (`PrimitiveComponent.SetPhysicsLinearVelocity` _staticmesh (.location (`|GetArrayItem` _actorvelocities_2 _returnvalue_4)) false "None")
          (`PrimitiveComponent.SetPhysicsAngularVelocityInDegrees` _staticmesh (.scale (`|GetArrayItem` _actorvelocities_2 _returnvalue_4)) false "None")
          (if (> _returnvalue_3 0)
            (`KismetArrayLibrary.Array_Remove` _actorvelocities _returnvalue_3)
            (else
              (`KismetArrayLibrary.Array_Clear` _actorvelocities))))
        (else
          (bind _returnvalue_5 (`PrimitiveComponent.GetPhysicsLinearVelocity` _staticmesh_2 "None"))
          (`KismetArrayLibrary.Array_Add` _actorvelocities_3 (`KismetMathLibrary.MakeTransform` _returnvalue_5 (struct) (`PrimitiveComponent.GetPhysicsAngularVelocityInDegrees` _staticmesh_2 "None")))
          (if (`self.ShouldDelete0thTerm`)
            (`KismetArrayLibrary.Array_Remove` _actorvelocities_3)))))))

(fn `ShouldDelete0thTerm`
  (returns (result :type Boolean))
  (bind _asbp_character (cast `/Game/Blueprints/Core/BP_Character` (`GameplayStatics.GetPlayerCharacter` 0))
    (:`then`
      (return (`/Game/Blueprints/Core/BP_Character.StartClearingOriginalTimePoints` _asbp_character)))
    (:`CastFailed`
      (return false))))

(fn `UserConstructionScript`
  (bind _staticmesh (`self.StaticMesh`))
  (`StaticMeshComponent.SetStaticMesh` _staticmesh (`self.Mesh`))
  (for (_array_element _array_index) (`self.Material`)
    (`PrimitiveComponent.SetMaterial` _staticmesh _array_index _array_element))
  (`PrimitiveComponent.SetSimulatePhysics` _staticmesh true))