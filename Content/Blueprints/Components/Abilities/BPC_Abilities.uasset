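; Player ability component that gives BP_Character active abilities, passive perks and a time-rewind ultimate.
; The selected Tree picks Dash or Invisibility, with clone spawning as a separate event.
; Hook events and query functions check the equipped passive or active ability to apply effects like regeneration, lifesteal, speed boosts and sixth-sense indicators.
; Rewind messages all BPI_TimeControl actors, then forwards them after a delay; its availability check always passes.
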(event `self.ReceiveBeginPlay`
  (bind _asbp_character (cast `/Game/Blueprints/Core/BP_Character` (`GameplayStatics.GetPlayerCharacter` 0)))
  (set `self.Character` _asbp_character))

(event `ActiveAbility`
  (switch `/Game/Blueprints/Components/Abilities/EAbilityTree` (`self.Tree`)
    (:`NewEnumerator0`
      (`self.Dash`))
    (:`NewEnumerator1`
      (`self.Invisibility`))))

(event `Dash`
  (bind _character (`self.Character`))
  (bind _character_2 (`self.Character`))
  (bind (_returnvalue_x _returnvalue_y _returnvalue_z) (`KismetMathLibrary.BreakVector` (`SceneComponent.GetForwardVector` (`/Game/Blueprints/Core/BP_Character.FirstPersonCamera` _character_2))))
  (bind _velocity (`MovementComponent.Velocity` (`Character.CharacterMovement` _character_2)))
  (if (> (`self.ActiveAbilityCharges`) 0)
    (bind _output_get (set `self.PreDashVelocity` _velocity))
    (`Character.LaunchCharacter` _character_2 (* (`KismetMathLibrary.MakeVector` _returnvalue_x _returnvalue_y (`KismetMathLibrary.FClamp` _returnvalue_z -0.5 0.5)) 2000.0) false true)
    (`/Game/Blueprints/Core/BP_Character.Dash_CameraFOV` _character)
    (`KismetSystemLibrary.Delay` 0.2)
    (`/Game/Blueprints/Core/BP_Character.Dash_SlowSpeed` _character _velocity (`KismetMathLibrary.FMin` (`KismetMathLibrary.VSize` _output_get) (`KismetMathLibrary.VSize` _velocity)))))

(event `Invisibility`
  (bind _character (`self.Character`))
  (`/Game/Blueprints/Core/BP_Character.StartInvisibility` _character)
  (`KismetSystemLibrary.Delay` 5.0)
  (`/Game/Blueprints/Core/BP_Character.EndInvisibility` _character))

(event `Rewind`
  (if (`self.CanUseUltimate`)
    (if (not (`self.Rewinding`))
      (set `self.Rewinding` true)
      (bind _outactors (`GameplayStatics.GetAllActorsWithInterface` "/Game/Blueprints/Components/Abilities/Ultimates/Rewind/BPI_TimeControl.BPI_TimeControl_C"))
      (for _array_element _outactors
        (message `/Game/Blueprints/Components/Abilities/Ultimates/Rewind/BPI_TimeControl.Rewind` _array_element))
      (`KismetSystemLibrary.Delay` 5.0)
      (bind _outactors_2 (`GameplayStatics.GetAllActorsWithInterface` "/Game/Blueprints/Components/Abilities/Ultimates/Rewind/BPI_TimeControl.BPI_TimeControl_C"))
      (for _array_element_2 _outactors_2
        (message `/Game/Blueprints/Components/Abilities/Ultimates/Rewind/BPI_TimeControl.Forward` _array_element_2))
      (set `self.Rewinding` false))))

(event `Event OnRegeneration`
  (bind _character (`self.Character`))
  (bind _character_2 (`self.Character`))
  (bind _currenthealth (`/Game/Blueprints/Core/BP_Character.CurrentHealth` _character))
  (bind _maxhealth (`/Game/Blueprints/Core/BP_Character.MaxHealth` _character))
  (bind _maxshield (`/Game/Blueprints/Core/BP_Character.MaxShield` _character))
  (`|ExecutionSequence`
    (:`then_0`
      (`self.IsCorrectPassive` "NewEnumerator1"
        (:`then`
          (set `/Game/Blueprints/Core/BP_Character.LagCurrentHealth` (`KismetMathLibrary.FClamp` (+ _currenthealth (`self.RegenerateAdd`)) 0.0 _maxhealth) _character)
          (bind _result (`/Engine/EditorBlueprintResources/StandardMacros.Float += Clamped` _currenthealth 0.25 0.0 _maxhealth)
            (:`  `
              (if (== _result _maxhealth)
                (`/Game/Blueprints/Core/BP_Character.RegenerationStop` _character_2)))))))
    (:`then_1`
      (`self.IsCorrectPassive` "NewEnumerator0"
        (:`then`
          (bind _result_2 (`/Engine/EditorBlueprintResources/StandardMacros.Float += Clamped` (`/Game/Blueprints/Core/BP_Character.CurrentShield` _character) 0.125 0.0 _maxshield)
            (:`  `
              (if (== _result_2 _maxshield)
                (`/Game/Blueprints/Core/BP_Character.RegenerationStop` _character_2)))))))))

(event `Event OnBulletBlocked`
  (bind _character (`self.Character`))
  (bind _returnvalue (+ 0.35 1.0))
  (bind _returnvalue_2 (+ 0.5 1.0))
  (bind _charactermovement (`Character.CharacterMovement` _character))
  (bind _parkourmovement (`/Game/Blueprints/Core/BP_Character.ParkourMovement` _character))
  (bind _defaultmaxwalkspeed (`/Game/Blueprints/Components/ParkourMovement.DefaultMaxWalkSpeed` _parkourmovement))
  (bind _sprintspeed (`/Game/Blueprints/Components/ParkourMovement.SprintSpeed` _parkourmovement))
  (bind _returnvalue_3 (`|EnumEquality` (`/Game/Blueprints/Components/ParkourMovement.CurrentParkourMode` _parkourmovement) "NewEnumerator4"))
  (`self.IsCorrectPassive` "NewEnumerator2"
    (:`then`
      (bind _output_get (set `/Game/Blueprints/Components/ParkourMovement.DefaultMaxWalkSpeed` (* _defaultmaxwalkspeed _returnvalue_2) _parkourmovement))
      (bind _output_get_2 (set `/Game/Blueprints/Components/ParkourMovement.SprintSpeed` (* _sprintspeed _returnvalue) _parkourmovement))
      (set `CharacterMovementComponent.MaxWalkSpeed` (select `bool` _returnvalue_3 :`false` _output_get :`true` _output_get_2) _charactermovement)
      (`KismetSystemLibrary.Delay` 2.0)
      (bind _output_get_3 (set `/Game/Blueprints/Components/ParkourMovement.DefaultMaxWalkSpeed` (/ _defaultmaxwalkspeed _returnvalue_2) _parkourmovement))
      (bind _output_get_4 (set `/Game/Blueprints/Components/ParkourMovement.SprintSpeed` (/ _sprintspeed _returnvalue) _parkourmovement))
      (set `CharacterMovementComponent.MaxWalkSpeed` (select `bool` _returnvalue_3 :`false` _output_get_3 :`true` _output_get_4) _charactermovement))))

(event `Event OnTakeDamage`
  (bind _activeabilityamountmax (`self.ActiveAbilityAmountMax`))
  (`self.IsCorrectPassive` "NewEnumerator3"
    (:`then`
      (`/Engine/EditorBlueprintResources/StandardMacros.Float += Clamped` (`self.CurrentActiveAbilityAmount`) (* _activeabilityamountmax 0.075) 0.0 _activeabilityamountmax))))

(event `UseClone`
  (bind _character (`self.Character`))
  (bind (_returnvalue_location _returnvalue_rotation) (`KismetMathLibrary.BreakTransform` (`Actor.GetTransform` _character)))
  (`|SpawnActorFromClass` "/Game/Blueprints/Components/Abilities/Actives/Clone/BP_Clone.BP_Clone_C" (`KismetMathLibrary.MakeTransform` (+ (* (`Actor.GetActorForwardVector` _character) 50.0) _returnvalue_location) _returnvalue_rotation) "Undefined" "OverrideRootScale" null null))

(event `Event OnDealDamage`
  (params (Amount :type "Float (double-precision)"))
  (bind _character (`self.Character`))
  (`self.IsCorrectActive` "NewEnumerator2"
    (:`then`
      (`/Engine/EditorBlueprintResources/StandardMacros.Float += Clamped` (`/Game/Blueprints/Core/BP_Character.CurrentHealth` _character) (/ Amount 2.0) 0.0 (`/Game/Blueprints/Core/BP_Character.MaxHealth` _character)))))

(fn `CanUseUltimate`
  (returns (` ` :type Boolean))
  (return true))

(fn `Event OnEnemyLock`
  (params (`Enemy Location` :type "Vector Structure"))
  (`self.IsCorrectPassive` "NewEnumerator8"
    (:`then`
      (bind _returnvalue (`|CreateWidget` "/Game/Blueprints/Components/Abilities/Passives/SixthSense/UI_SixthSenseDirection.UI_SixthSenseDirection_C" null (- (.yaw (`KismetMathLibrary.FindLookAtRotation` (`KismetMathLibrary.MakeVector` (.x (`Actor.K2_GetActorLocation` (`self.Character`))) (.y (`Actor.K2_GetActorLocation` (`self.Character`)))) (`KismetMathLibrary.MakeVector` (.x `Enemy Location`) (.y `Enemy Location`)))) (.yaw (`Actor.K2_GetActorRotation` (`self.Character`))))))
      (`UserWidget.AddToViewport` _returnvalue 0))))

(fn `GetDamageMultipliers`
  (returns (`%` :type "Float (double-precision)"))
  (`|ExecutionSequence`
    (:`then_0`
      (`self.IsCorrectActive` "NewEnumerator6"
        (:`then`
          (return 0.5))))
    (:`then_1`
      (return 1.0))))

(fn `GetReloadSpeed`
  (returns (ReloadSpeed :type "Float (double-precision)"))
  (`self.IsCorrectPassive` "NewEnumerator4"
    (:`then`
      (return (* 1.0 2.0)))
    (:`Fail`
      (return 1.0))))

(fn `GetStepSound`
  (returns (Sound :type "Float (double-precision)"))
  (`self.IsCorrectPassive` "NewEnumerator6"
    (:`then`
      (return 0.0))
    (:`Fail`
      (return 1.0))))

(fn `ShouldSeeEnemyFootprints`
  (returns (_ :type Boolean))
  (`self.IsCorrectPassive` "NewEnumerator9"
    (:`then`
      (return true))
    (:`Fail`
      (return false))))

(fn `ShouldTakeFallDamage`
  (returns (_ :type Boolean))
  (`self.IsCorrectPassive` "NewEnumerator7"
    (:`then`
      (return true))
    (:`Fail`
      (return false))))

(fn `SwitchTree`
  (params (NewTree :type "/Game/Blueprints/Components/Abilities/EAbilityTree Enum" :default "NewEnumerator0"))
  (bind _output_get (set `self.Tree` NewTree))
  (switch `/Game/Blueprints/Components/Abilities/EAbilityTree` _output_get
    (:`NewEnumerator0`
      (set `self.MaxActiveAbilityCharges` 2))))