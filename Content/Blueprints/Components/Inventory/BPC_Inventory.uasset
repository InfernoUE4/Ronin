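; Inventory component that tracks pickup items near the player and adds them to the stored inventory.
; On BeginPlay it caches BP_Character and its NearbyItems; UpdateNearbyItems maps overlapping BP_BaseItems by item data and flags a refresh, which GetNearbyItems returns with the keys.
; AddItem merges by whole stack or single unit, matching quality, item and per-item weight, otherwise appending an entry.
; World actors are destroyed only on certain merge paths, not when appending.
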(event `self.ReceiveBeginPlay`
  (bind _asbp_character (cast `/Game/Blueprints/Core/BP_Character` (`GameplayStatics.GetPlayerCharacter` 0)))
  (bind _output_get (set `self.Character` _asbp_character))
  (set `self.Nearby Items` (`/Game/Blueprints/Core/BP_Character.NearbyItems` _output_get)))

(fn `AddItem`
  (params (`Add Type` :type "/Game/Blueprints/Components/Inventory/EAddItemType Enum" :default "NewEnumerator0") (`Item Data` :type "/Game/Blueprints/Components/Inventory/ST_ItemData Structure"))
  (returns (Result :type Boolean))
  (bind ((`Amount_14_6E07844841B66812CF8544B0F8FA5721` _amount)) (break `/Game/Blueprints/Components/Inventory/ST_ItemData` `Item Data`))
  (bind (_name _itemquality _itemtype _item _amount_2 _peritemweight _canstack) (break `/Game/Blueprints/Components/Inventory/ST_ItemData` `Item Data`))
  (bind _inventory (`self.Inventory`))
  (bind (_value _returnvalue) (`BlueprintMapLibrary.Map_Find` (`self.NearbyItems`) `Item Data`))
  (switch `/Game/Blueprints/Components/Inventory/EAddItemType` `Add Type`
    (:`NewEnumerator0`
      (for _array_element _inventory
        (if (`self.Item ==` _array_element `Item Data`)
          (`/Engine/EditorBlueprintResources/StandardMacros.Integer +=` (`.Amount_14_6E07844841B66812CF8544B0F8FA5721` (break `/Game/Blueprints/Components/Inventory/ST_ItemData` _array_element)) (`.Amount_14_6E07844841B66812CF8544B0F8FA5721` (break `/Game/Blueprints/Components/Inventory/ST_ItemData` `Item Data`))
            (:`  `
              (if _returnvalue
                (`Actor.K2_DestroyActor` _value)
                (return true)
                (else
                  (`KismetSystemLibrary.PrintString` "Error Destroying Actor After Add" true true (struct :`R` 1.0 :`A` 1.0) 10.0)
                  (return false)))))))
      (`KismetArrayLibrary.Array_Add` (`self.Inventory`) `Item Data`))
    (:`NewEnumerator1`
      (for _array_element_2 _inventory
        (if (`self.Item ==` _array_element_2 `Item Data`)
          (`/Engine/EditorBlueprintResources/StandardMacros.IncrementInt` (`.Amount_14_6E07844841B66812CF8544B0F8FA5721` (break `/Game/Blueprints/Components/Inventory/ST_ItemData` _array_element_2))
            (:`  `
              (`/Engine/EditorBlueprintResources/StandardMacros.DecrementInt` _amount
                (:`  `
                  (if (< _amount 0)
                    (if _returnvalue
                      (`Actor.K2_DestroyActor` _value)
                      (return true)))))))))
      (`KismetArrayLibrary.Array_Add` (`self.Inventory`) (make `/Game/Blueprints/Components/Inventory/ST_ItemData` _name _itemquality _itemtype _item 1 _peritemweight _canstack)))))

(fn `GetNearbyItems`
  (returns (NearbyItems :type "Array of /Game/Blueprints/Components/Inventory/ST_ItemData Structure") (ShouldUpdateNearbyItems :type Boolean))
  (bind _keys (`BlueprintMapLibrary.Map_Keys` (`self.NearbyItems`)))
  (return _keys (`self.ShouldUpdateNearbyItems`)))

(fn `Item ==`
  (params (` ` :type "/Game/Blueprints/Components/Inventory/ST_ItemData Structure") (`  ` :type "/Game/Blueprints/Components/Inventory/ST_ItemData Structure"))
  (returns (`   ` :type Boolean))
  (bind (_name _itemquality _itemtype _item _amount _peritemweight) (break `/Game/Blueprints/Components/Inventory/ST_ItemData` `  `))
  (bind (_name_2 _itemquality_2 _itemtype_2 _item_2 _amount_2 _peritemweight_2) (break `/Game/Blueprints/Components/Inventory/ST_ItemData` ` `))
  (return (and (`|EnumEquality` _itemquality_2 _itemquality) (`|EnumEquality` _item_2 _item) (== _peritemweight_2 _peritemweight))))

(fn `UpdateNearbyItems`
  (`BlueprintMapLibrary.Map_Clear` (`self.NearbyItems`))
  (for _array_element (`PrimitiveComponent.GetOverlappingActors` (`self.Nearby Items`) null)
    (bind _asbp_base_item (cast `/Game/Blueprints/Components/Inventory/BP_BaseItem` _array_element))
    (`BlueprintMapLibrary.Map_Add` (`self.NearbyItems`) (`/Game/Blueprints/Components/Inventory/BP_BaseItem.ItemData` _asbp_base_item) _asbp_base_item))
  (set `self.ShouldUpdateNearbyItems` true))