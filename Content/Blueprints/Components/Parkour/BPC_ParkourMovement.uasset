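; Parkour component that adds sprint, crouch, slide, wall run, mantle and multi-jump to a character.
; A movement-state enum drives it: each change resets prior modes, while Tick traces for walls and ledges and runs the active state.
; Wall runs and mantles use launches; slides use an impulse, zero friction, a plane constraint and slope-based braking.
; Actions fire paired Server and Client events, and debug prints and traces remain active.
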(event `Initialize`
  (params (Character :type "/Game/Blueprints/Core/BP_Character Object Reference"))
  (bind _charactermovement (`self.CharacterMovement`))
  (bind _output_get (set `self.Character` Character))
  (set `self.CharacterMovement` (`Character.CharacterMovement` _output_get))
  (set `self.Default_WalkSpeed` (`CharacterMovementComponent.MaxWalkSpeed` _charactermovement))
  (set `self.Default_WalkSpeed_Crouched` (`CharacterMovementComponent.MaxWalkSpeedCrouched` _charactermovement))
  (set `self.Default_GroundFriction` (`CharacterMovementComponent.GroundFriction` _charactermovement))
  (set `self.Default_DecelerationWalking` (`CharacterMovementComponent.BrakingDecelerationWalking` _charactermovement)))

(event `StartSprint`
  (`self.UpdateMovement` "NewEnumerator1")
  (`self.StartSprint (Server)`)
  (`self.StartSprint (Client)`))

(event `StartSprint (Server)`
  (set `CharacterMovementComponent.MaxWalkSpeed` (`self.SprintSpeed`) (`self.CharacterMovement`)))

(event `StartSprint (Client)`
  (set `CharacterMovementComponent.MaxWalkSpeed` (`self.SprintSpeed`) (`self.CharacterMovement`)))

(event `EndSprint (Server)`
  (set `CharacterMovementComponent.MaxWalkSpeed` (`self.Default_WalkSpeed`) (`self.CharacterMovement`)))

(event `EndSprint (Client)`
  (set `CharacterMovementComponent.MaxWalkSpeed` (`self.Default_WalkSpeed`) (`self.CharacterMovement`)))

(event `EndSprint`
  (`self.UpdateMovement` "NewEnumerator0")
  (`self.ResetSprint`))

(event `SprintToggle`
  (if (`|EnumEquality` (`self.CurrMovement`) "NewEnumerator1")
    (`self.EndSprint`)
    (else
      (`self.StartSprint`))))

(event `ResetSprint`
  (`self.EndSprint (Server)`)
  (`self.EndSprint (Client)`))

(event `StartCrouch`
  (if (`|EnumInequality` (`self.CurrMovement`) "NewEnumerator1")
    (`self.UpdateMovement` "NewEnumerator2")
    (`self.StartCrouch (Server)`)
    (`self.StartCrouch (Client)`)
    (else
      (`self.StartSlide`))))

(event `StartCrouch (Server)`
  (`Character.Crouch` (`self.Character`)))

(event `StartCrouch (Client)`
  (`Character.Crouch` (`self.Character`)))

(event `EndCrouch (Server)`
  (`Character.UnCrouch` (`self.Character`)))

(event `EndCrouch (Client)`
  (`Character.UnCrouch` (`self.Character`)))

(event `EndCrouch`
  (`self.UpdateMovement` "NewEnumerator0")
  (`self.ResetCrouch`))

(event `CrouchToggle`
  (if (`|EnumEquality` (`self.CurrMovement`) "NewEnumerator2")
    (`self.EndCrouch`)
    (else
      (`self.StartCrouch`))))

(event `ResetCrouch`
  (`self.EndCrouch (Server)`)
  (`self.EndCrouch (Client)`))

(event `StartSlide`
  (`self.UpdateMovement` "NewEnumerator3")
  (`self.StartSlide (Server)`)
  (`self.StartSlide (Client)`))

(event `StartSlide (Server)`
  (bind _charactermovement (`self.CharacterMovement`))
  (bind _returnvalue (`Actor.K2_GetActorLocation` (`self.Character`)))
  (bind (_outhit _returnvalue_2) (`KismetSystemLibrary.LineTraceSingle` :`Start` _returnvalue :`End` (- _returnvalue (0.0 0.0 200.0)) :`TraceChannel` "TraceTypeQuery1" :`DrawDebugType` "ForDuration"))
  (if _returnvalue_2
    (bind (_bblockinghit _binitialoverlap _time _distance _location _impactpoint _normal _impactnormal) (`GameplayStatics.BreakHitResult` _outhit))
    (bind _returnvalue_3 (+ (* (/ (* (.z (* (`KismetMathLibrary.Cross_VectorVector` _impactnormal (`Actor.GetActorRightVector` (`self.Character`))) -1.0)) 1.0) (/ 1.0 3.0)) 1400.0) 1400.0))
    (bind _output_get (set `self.WalkingDeceleration (Sliding)` (`KismetMathLibrary.FClamp` _returnvalue_3 0.0 _returnvalue_3)))
    (set `CharacterMovementComponent.BrakingDecelerationWalking` _output_get (`self.CharacterMovement`))
    (set `CharacterMovementComponent.GroundFriction` 0.0 (`self.CharacterMovement`)) ; 0 Friction for slipping and sliding
    (set `CharacterMovementComponent.MaxWalkSpeedCrouched` 0.0 _charactermovement) ; Stop player from controlling slide once initiated
    (bind _output_get_2 (set `self.SlideVelocityNormal` (`KismetMathLibrary.Normal` (`MovementComponent.Velocity` _charactermovement))))
    (`MovementComponent.SetPlaneConstraintFromVectors` _charactermovement _output_get_2 (`Actor.GetActorUpVector` (`self.Character`)))
    (`MovementComponent.SetPlaneConstraintEnabled` _charactermovement true)
    (bind _output_get_3 (set `self.SlideImpulse` (* (`KismetMathLibrary.Cross_VectorVector` _impactnormal (`Actor.GetActorRightVector` (`self.Character`))) -900.0)))
    (`CharacterMovementComponent.AddImpulse` (`self.CharacterMovement`) _output_get_3 true)
    (`Character.Crouch` (`self.Character`))
    (else
      (`self.UpdateMovement` "NewEnumerator0"))))

(event `StartSlide (Client)`
  (bind _charactermovement (`self.CharacterMovement`))
  (bind _charactermovement_2 (`self.CharacterMovement`))
  (set `CharacterMovementComponent.GroundFriction` 0.0 _charactermovement_2) ; 0 Friction for slipping and sliding
  (set `CharacterMovementComponent.MaxWalkSpeedCrouched` 0.0 _charactermovement_2) ; Stop player from controlling slide once initiated
  (`MovementComponent.SetPlaneConstraintFromVectors` _charactermovement (`self.SlideVelocityNormal`) (`Actor.GetActorUpVector` (`self.Character`)))
  (`MovementComponent.SetPlaneConstraintEnabled` _charactermovement true)
  (if (not (`KismetSystemLibrary.IsServer`))
    (`CharacterMovementComponent.AddImpulse` (`self.CharacterMovement`) (`self.SlideImpulse`) true)
    (`Character.Crouch` (`self.Character`))))

(event `EndSlide (Server)`
  (bind _charactermovement (`self.CharacterMovement`))
  (set `CharacterMovementComponent.MaxWalkSpeed` (`self.Default_WalkSpeed`) _charactermovement)
  (set `CharacterMovementComponent.MaxWalkSpeedCrouched` (`self.Default_WalkSpeed_Crouched`) _charactermovement)
  (set `CharacterMovementComponent.GroundFriction` (`self.Default_GroundFriction`) _charactermovement)
  (set `CharacterMovementComponent.BrakingDecelerationWalking` (`self.Default_DecelerationWalking`) _charactermovement)
  (`MovementComponent.SetPlaneConstraintEnabled` _charactermovement false))

(event `EndSlide (Client)`
  (bind _charactermovement (`self.CharacterMovement`))
  (set `CharacterMovementComponent.MaxWalkSpeed` (`self.Default_WalkSpeed`) _charactermovement)
  (set `CharacterMovementComponent.MaxWalkSpeedCrouched` (`self.Default_WalkSpeed_Crouched`) _charactermovement)
  (set `CharacterMovementComponent.GroundFriction` (`self.Default_GroundFriction`) _charactermovement)
  (set `CharacterMovementComponent.BrakingDecelerationWalking` (`self.Default_DecelerationWalking`) _charactermovement)
  (`MovementComponent.SetPlaneConstraintEnabled` _charactermovement false))

(event `EndSlide`
  (`self.UpdateMovement` "NewEnumerator0")
  (`self.ResetCrouch`))

(event `ResetSlide`
  (`self.EndSlide (Server)`)
  (`self.EndSlide (Client)`))

(event `UpdateMovement`
  (params (NewMovement :type "/Game/Blueprints/Components/Parkour/EParkourMode Enum" :default "NewEnumerator0"))
  (set `self.PrevMovement` (`self.CurrMovement`))
  (set `self.CurrMovement` NewMovement)
  (`self.ResetAllCurrent`))

(event `ResetAllCurrent`
  (`self.ResetCrouch`)
  (`self.ResetSprint`)
  (`self.ResetSlide`)
  (set `self.ShouldMantle` false))

(event `self.ReceiveTick`
  (params (DeltaSeconds :type "Float (single-precision)"))
  (bind _character (`self.Character`))
  (bind _sprintspeed (`self.SprintSpeed`))
  (bind _sprintspeed_2 (`self.SprintSpeed`))
  (bind _character_2 (`self.Character`))
  (bind _array (`|MakeArray` _character :!type "Actor Object Reference"))
  (bind _capsulecomponent (`Character.CapsuleComponent` (`self.Character`)))
  (bind _returnvalue (`SceneComponent.K2_GetComponentLocation` (`/Game/Blueprints/Core/BP_Character.WallRun_L` _character)))
  (bind _returnvalue_2 (`SceneComponent.K2_GetComponentLocation` (`/Game/Blueprints/Core/BP_Character.WallRun_R` (`self.Character`))))
  (bind _capsulehalfheight (`CapsuleComponent.CapsuleHalfHeight` _capsulecomponent))
  (bind _returnvalue_3 (`KismetMathLibrary.MakeVector` 0.0 0.0 _capsulehalfheight))
  (bind _returnvalue_4 (+ (`Actor.K2_GetActorLocation` _character_2) (* (`Actor.GetActorForwardVector` _character_2) 100.0)))
  (`KismetSystemLibrary.PrintString` (`KismetStringLibrary.Concat_StrStr` "C: " (`|GetEnumeratorNameAsString` (`self.CurrMovement`)) "P: " (`|GetEnumeratorNameAsString` (`self.PrevMovement`))) true true (struct :`G` 0.66 :`B` 1.0 :`A` 1.0) DeltaSeconds)
  (`|ExecutionSequence`
    (:`then_0`
      (`|ExecutionSequence`
        (:`then_0`
          (if (`NavMovementComponent.IsFalling` (`self.CharacterMovement`))
            (`|ExecutionSequence`
              (:`then_0`
                (bind (_outhit _returnvalue_5) (`KismetSystemLibrary.SphereTraceSingle` _returnvalue_2 _returnvalue_2 20.0 "TraceTypeQuery1" true _array "ForDuration"))
                (if _returnvalue_5
                  (`self.UpdateMovement` "NewEnumerator4")
                  (set `self.WallRunVelocity` (* (`KismetMathLibrary.Cross_VectorVector` (`.ImpactNormal` (`GameplayStatics.BreakHitResult` _outhit)) (0.0 0.0 1.0)) (* (`KismetMathLibrary.FMax` (`KismetMathLibrary.SelectFloat` (* _sprintspeed_2 1.5) (* _sprintspeed_2 1.0) (`|EnumEquality` (`self.PrevMovement`) "NewEnumerator1")) (`KismetMathLibrary.VSize` (`Actor.GetVelocity` (`self.Character`)))) -1.0)))
                  (elif (`|EnumEquality` (`self.CurrMovement`) "NewEnumerator4")
                    (`self.UpdateMovement` "NewEnumerator0"))))
              (:`then_1`
                (bind (_outhit_2 _returnvalue_6) (`KismetSystemLibrary.SphereTraceSingle` _returnvalue _returnvalue 20.0 "TraceTypeQuery1" true _array "ForDuration"))
                (if _returnvalue_6
                  (`self.UpdateMovement` "NewEnumerator5")
                  (set `self.WallRunVelocity` (* (`KismetMathLibrary.Cross_VectorVector` (`.ImpactNormal` (`GameplayStatics.BreakHitResult` _outhit_2)) (0.0 0.0 1.0)) (* (`KismetMathLibrary.FMax` (`KismetMathLibrary.SelectFloat` (* _sprintspeed 1.5) (* _sprintspeed 1.0) (`|EnumEquality` (`self.PrevMovement`) "NewEnumerator1")) (`KismetMathLibrary.VSize` (`Actor.GetVelocity` (`self.Character`)))) 1.0)))
                  (elif (`|EnumEquality` (`self.CurrMovement`) "NewEnumerator5")
                    (`self.UpdateMovement` "NewEnumerator0")))))))
        (:`then_1`
          (if (`|EnumInequality` (`self.CurrMovement`) "NewEnumerator6")
            (set `self.ShouldMantle` false)
            (if (`NavMovementComponent.IsFalling` (`self.CharacterMovement`))
              (bind (_outhit_3 _returnvalue_7) (`KismetSystemLibrary.LineTraceSingle` (+ _returnvalue_4 (0.0 0.0 125.0)) (- _returnvalue_4 (0.0 0.0 0.0)) "TraceTypeQuery1" true))
              (if _returnvalue_7
                (bind (_bblockinghit _binitialoverlap _time _distance _location) (`GameplayStatics.BreakHitResult` _outhit_3))
                (bind _returnvalue_8 (+ _location _returnvalue_3 (0.0 0.0 10.0)))
                (bind (_outhit_4 _returnvalue_9) (`KismetSystemLibrary.CapsuleTraceSingle` :`Start` _returnvalue_8 :`End` _returnvalue_8 :`Radius` (`CapsuleComponent.CapsuleRadius` _capsulecomponent) :`HalfHeight` (- _capsulehalfheight 5.0) :`TraceChannel` "TraceTypeQuery1" :`DrawDebugType` "ForDuration"))
                (if (not _returnvalue_9)
                  (set `self.MantleToPoint` (+ _location _returnvalue_3))
                  (`self.UpdateMovement` "NewEnumerator6"))))))))
    (:`then_1`
      (switch `/Game/Blueprints/Components/Parkour/EParkourMode` (`self.CurrMovement`)
        (:`NewEnumerator1`
          (if (< (`/Game/Blueprints/Core/BP_Character.GetMovementInputs` (`self.Character`)) 0.9)
            (`self.UpdateMovement` "NewEnumerator0")))
        (:`NewEnumerator2`
          (if (`NavMovementComponent.IsFalling` (`self.CharacterMovement`))
            (`self.UpdateMovement` "NewEnumerator0")))
        (:`NewEnumerator3`
          (`self.SlidingTick (Server)`)
          (`self.SlidingTick (Client)`))
        (:`NewEnumerator4`
          (`self.WallRunning (Server)` :!label _label)
          (`self.WallRunning (Client)`))
        (:`NewEnumerator5`
          (goto _label))
        (:`NewEnumerator6`
          (`self.Mantle (Parkour)`))))))

(event `SlidingTick (Client)`
  (set `CharacterMovementComponent.BrakingDecelerationWalking` (`self.WalkingDeceleration (Sliding)`) (`self.CharacterMovement`)))

(event `SlidingTick (Server)`
  (bind _returnvalue (`Actor.K2_GetActorLocation` (`self.Character`)))
  (bind (_outhit _returnvalue_2) (`KismetSystemLibrary.LineTraceSingle` :`Start` _returnvalue :`End` (- _returnvalue (0.0 0.0 200.0)) :`TraceChannel` "TraceTypeQuery1" :`DrawDebugType` "ForDuration"))
  (if _returnvalue_2
    (if (> (`KismetMathLibrary.VSize` (`MovementComponent.Velocity` (`self.CharacterMovement`))) 300.0)
      (bind _returnvalue_3 (+ (* (/ (* (.z (* (`KismetMathLibrary.Cross_VectorVector` (`.ImpactNormal` (`GameplayStatics.BreakHitResult` _outhit)) (`Actor.GetActorRightVector` (`self.Character`))) -1.0)) 1.0) (/ 1.0 3.0)) 1400.0) 1400.0))
      (bind _output_get (set `self.WalkingDeceleration (Sliding)` (`KismetMathLibrary.FClamp` _returnvalue_3 0.0 _returnvalue_3)))
      (set `CharacterMovementComponent.BrakingDecelerationWalking` _output_get (`self.CharacterMovement`))
      (else
        (`self.UpdateMovement` "NewEnumerator0" :!label _label_2)))
    (else
      (goto _label_2))))

(event `WallRunning (Client)`
  (`Character.LaunchCharacter` (`self.Character`) (`self.WallRunVelocity`) true true))

(event `WallRunning (Server)`
  (`Character.LaunchCharacter` (`self.Character`) (`self.WallRunVelocity`) true true))

(event `Mantle (Parkour)`
  (`self.Mantle (Server)`)
  (`self.Mantle (Client)`))

(event `Mantle (Server)`
  (bind _output_get (set `self.ShouldMantle` (> (.z (`self.MantleToPoint`)) (.z (`Actor.K2_GetActorLocation` (`self.Character`))))))
  (if _output_get
    (`Character.LaunchCharacter` (`self.Character`) (0.0 0.0 200.0) true true)
    (`KismetSystemLibrary.PrintString` "Hello")))

(event `Mantle (Client)`
  (if (`self.ShouldMantle`)
    (`Character.LaunchCharacter` (`self.Character`) (0.0 0.0 200.0) true true)
    (else
      (`self.UpdateMovement` "NewEnumerator0"))))

(event `Jump`
  (bind _jumpcount (`self.JumpCount`))
  (if (> (`self.MaxJumpCount`) _jumpcount)
    (`/Engine/EditorBlueprintResources/StandardMacros.IncrementInt` _jumpcount
      (:`  `
        (`self.UpdateMovement` "NewEnumerator0")
        (`self.Jump (Server)`)
        (`self.Jump (Client)`)))))

(event `Jump (Client)`
  (if (not (`KismetSystemLibrary.IsServer`))
    (`Character.LaunchCharacter` (`self.Character`) (`self.JumpVelocity`) false true)))

(event `Event OnLanded`
  (set `self.JumpCount` 0))

(event `Jump (Server)`
  (bind _character (`self.Character`))
  (bind (_f_b _r_l) (`/Game/Blueprints/Core/BP_Character.GetMovementInputs` _character))
  (bind _returnvalue (/ (`self.JumpZVelocity`) 6.0))
  (`KismetSystemLibrary.PrintString` (`KismetStringLibrary.Concat_StrStr` (`KismetStringLibrary.Conv_DoubleToString` _f_b) " " (`KismetStringLibrary.Conv_DoubleToString` _r_l)))
  (bind _output_get (set `self.JumpVelocity` (`KismetMathLibrary.MakeVector` (.x (+ (* (`Actor.GetActorForwardVector` _character) (* _f_b _returnvalue)) (* (`Actor.GetActorRightVector` _character) (* _r_l _returnvalue)))) (.y (+ (* (`Actor.GetActorForwardVector` _character) (* _f_b _returnvalue)) (* (`Actor.GetActorRightVector` _character) (* _r_l _returnvalue)))) (`self.JumpZVelocity`))))
  (`Character.LaunchCharacter` (`self.Character`) _output_get false true))