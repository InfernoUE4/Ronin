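; Anim notify state that marks the window in an animation during which the character's katana trail is active.
; On begin it casts the mesh owner to BP_Character and sets its KatanaTrail flag to true; on end it sets the flag back to false.
; Both events return whether the cast succeeded, and the trail effect itself is handled outside this asset.
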(fn `Received_NotifyBegin`
  (params (MeshComp :type "SkeletalMeshComponent Object Reference") (Animation :type "AnimSequenceBase Object Reference") (TotalDuration :type "Float (double-precision)"))
  (returns (ReturnValue :type Boolean))
  (bind _asbp_character (cast `/Game/Blueprints/Core/BP_Character` (`ActorComponent.GetOwner` MeshComp))
    (:`then`
      (set `/Game/Blueprints/Core/BP_Character.KatanaTrail` true _asbp_character)
      (return true))
    (:`CastFailed`
      (return false))))

(fn `Received_NotifyEnd`
  (params (MeshComp :type "SkeletalMeshComponent Object Reference") (Animation :type "AnimSequenceBase Object Reference"))
  (returns (ReturnValue :type Boolean))
  (bind _asbp_character (cast `/Game/Blueprints/Core/BP_Character` (`ActorComponent.GetOwner` MeshComp))
    (:`then`
      (set `/Game/Blueprints/Core/BP_Character.KatanaTrail` false _asbp_character)
      (return true))
    (:`CastFailed`
      (return false))))